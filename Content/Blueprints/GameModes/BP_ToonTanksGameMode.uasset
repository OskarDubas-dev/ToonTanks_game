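; Game mode Blueprint for ToonTanks that shows the start and game-over screens.
; StartGame adds the start widget to the viewport, and GameOver adds the end widget with a win or loss message chosen by a Select on WonGame.
; An equivalent Branch version of the text choice is left unconnected.
; Background music on BeginPlay sits behind an always-false condition, so it never plays.
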(event EventBeginPlay
  (if false
    (Audio|PlaySound2D "/Game/Assets/Audio/BGM/BGM.BGM" 1.0 1.0 0.0 0 0)))

(event EventStartGame
  (bind _returnvalue (UserInterface|CreateWidget "/Game/Blueprints/Widgets/WBP_StartGameWidget.WBP_StartGameWidget_C"))
  (UserInterface|Viewport|AddtoViewport _returnvalue 0))

(event EventGameOver
  (params (bWonGame :type Boolean))
  (bind _returnvalue (UserInterface|CreateWidget "/Game/Blueprints/Widgets/WBP_GameOverWidget.WBP_GameOverWidget_C"))
  (UserInterface|Viewport|AddtoViewport _returnvalue 0)
  ;[1 1 1] Select way of doing this (better)
  (Rendering|Components|TextRender|SetText (Variables|/Game/Blueprints/Widgets/WBP_GameOverWidget.WBP_GameOverWidget_C|GetDisplayText _returnvalue) (select bWonGame "Clear!" "Game Over!")))

(fn ConstructionScript)